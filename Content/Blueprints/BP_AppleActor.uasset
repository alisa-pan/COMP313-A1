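; BP_AppleActor is an apple that BP_MyCharacter eats in two bites by bumping into it.
; Each mesh hit from the character counts after a short delay: the first plays a bite sound and swaps to a half-apple mesh, the second plays a chew sound and destroys the actor.
; Each bite adds half an apple to the character's ApplesEaten.
; A hit from a BP_NPC destroys the apple outright.
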(event `self.StaticMesh.OnComponentHit`
  (params (HitComponent :type "PrimitiveComponent Object Reference") (OtherActor :type "Actor Object Reference") (OtherComp :type "PrimitiveComponent Object Reference") (NormalImpulse :type "Vector Structure") (Hit :type "HitResult Structure (by ref)"))
  (bind _asbp_my_character (cast `/Game/Blueprints/BP_MyCharacter` OtherActor)
    (:`then`
      (`KismetSystemLibrary.Delay` 0.2)
      (bind _result (`/Engine/EditorBlueprintResources/StandardMacros.IncrementInt` (`self.crowHits`))
        (:`  `
          (if (== _result 1)
            (`GameplayStatics.PlaySound2D` "/Game/Audio/FOODEat_Apple_bite.FOODEat_Apple_bite" 1.0 1.0 0.0 null null)
            (`StaticMeshComponent.SetStaticMesh` (`self.StaticMesh`) "/Game/Food_Pack_01/Meshes/Food_Fruit_Apple_01_Half_01.Food_Fruit_Apple_01_Half_01")
            (set `MyCharacter.ApplesEaten` (+ (`MyCharacter.ApplesEaten` _asbp_my_character) 0.5) _asbp_my_character :!label _label)
            (elif (== (`self.crowHits`) 2)
              (`GameplayStatics.PlaySound2D` "/Game/Audio/FOODEat_Apple_chew.FOODEat_Apple_chew" 1.0 1.0 0.0 null null)
              (`self.K2_DestroyActor`)
              (goto _label))))))
    (:`CastFailed`
      (cast `/Game/Blueprints/BP_NPC` OtherActor)
      (`self.K2_DestroyActor`))))

(fn `UserConstructionScript`)