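; BP_NPC is a computer-controlled character that wanders between randomly chosen BP_AppleActor instances using AI MoveTo.
; Tick and a delayed BeginPlay share one chain that gathers all apples, waits a random few seconds, then moves to one.
; Tick bypasses the intended player headstart, with the random Delay pacing retargeting.
; The random index uses Length minus one as its exclusive maximum, so the last apple is excluded.
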(event `self.ReceiveBeginPlay`
  ;[1 1 1] Give player 3-second headstart at beginning of game
  (`KismetSystemLibrary.Delay` 3.0)
  ;[1 1 1] At every tick, get a random AppleActor from all the AppleActors in the game and move towards it
  (bind _outactors (`GameplayStatics.GetAllActorsOfClass` "/Game/Blueprints/BP_AppleActor.BP_AppleActor_C" :!label _label))
  ;[1 1 1] Wait between 1 to 5 seconds before next movement
  (`KismetSystemLibrary.Delay` (`KismetMathLibrary.RandomFloatInRange` 1.0 5.0))
  (`|AIMoveTo` self (0.0 0.0 0.0) (`|GetArrayItem` _outactors (`KismetMathLibrary.RandomInteger` (- (`KismetArrayLibrary.Array_Length` _outactors) 1)))))

(event `self.ReceiveTick`
  (params (DeltaSeconds :type "Float (single-precision)"))
  ;[1 1 1] At every tick, get a random AppleActor from all the AppleActors in the game and move towards it
  (goto _label))

(fn `UserConstructionScript`)