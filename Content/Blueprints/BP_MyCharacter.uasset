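; BP_MyCharacter is a character Blueprint that puts a HUD on screen and reacts to bumping into NPCs.
; On BeginPlay it creates the HUD widget, stores it in HudRef and adds it to the viewport.
; When a hit involves a BP_NPC, it moves itself without sweep to its own location with X and Y swapped, keeping height, rotation and scale.
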(event `self.ReceiveBeginPlay`
  (bind _returnvalue (`|CreateWidget` "/Game/UI_Widgets/HUD.HUD_C"))
  (bind _output_get (set `self.hudRef` _returnvalue))
  (`UserWidget.AddToViewport` _output_get 0))

(event `self.ReceiveHit`
  (params (MyComp :type "PrimitiveComponent Object Reference") (Other :type "Actor Object Reference") (OtherComp :type "PrimitiveComponent Object Reference") (bSelfMoved :type Boolean) (HitLocation :type "Vector Structure") (HitNormal :type "Vector Structure") (NormalImpulse :type "Vector Structure") (Hit :type "HitResult Structure (by ref)"))
  (cast `/Game/Blueprints/BP_NPC` Other)
  (`self.K2_SetActorTransform` (`KismetMathLibrary.MakeTransform` (`KismetMathLibrary.MakeVector` (.y (.location (`self.GetTransform`))) (.x (.location (`self.GetTransform`))) (.z (.location (`self.GetTransform`)))) (.rotation (`self.GetTransform`)) (.scale (`self.GetTransform`)))))

(fn `UserConstructionScript`)